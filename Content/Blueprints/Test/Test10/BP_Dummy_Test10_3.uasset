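; BP_Dummy_Test10_3 is a test dummy that reacts to damage by printing debug info and spawning a damage popup.
; AnyDamage prints the amount, instigator and causer, then spawns an actor of the class held in NewVar at the Scene component's world transform.
; The damage goes into the spawn through the exposed Danage property, then the actor's name is printed and OnPopupStart is called on it.
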(event Game|Damage|EventAnyDamage
  (params (Damage :type Float%20%28single-precision%29) (DamageType :type Damage%20Type%20Object%20Reference) (InstigatedBy :type Controller%20Object%20Reference) (DamageCauser :type Actor%20Object%20Reference))
  (Development|PrintString (Utilities|String|BuildString(Object) (Utilities|String|BuildString(Object) (Class|KismetStringLibrary|BuildStringDouble "" "Damage: " Damage) "Instigator" InstigatedBy) "Cause" DamageCauser))
  (bind _returnvalue (Game|SpawnActorfromClass (Variables|Default|GetNewVar) (Transformation|GetWorldTransform (Variables|Default|GetScene)) "Undefined" "MultiplyWithRoot" 0 Damage 0))
  (Development|PrintString (Utilities|GetDisplayName _returnvalue))
  (Class|DamagepopupActor|OnPopupStart _returnvalue 0.0))

(fn ConstructionScript)