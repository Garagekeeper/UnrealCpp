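; BP_CommandTest is a test Blueprint that issues inventory commands to the player's inventory component.
; On BeginPlay it casts the player pawn to BP_Test16Char2 and caches its InvenComponent.
; Separate events for Add, Move, Drop and Money pass its variables into a single ExecuteCommand call on that component, selected by command type.
; Drop also supplies the pawn's current location as the 3D target position.
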(event Custom|CommandMoney
  (Class|InventoryComponent|ExecuteCommand (Variables|Default|GetInven%20Component) (Utilities|Struct|MakeInventoryCommand "Money" (Variables|CommandTestMoney|GetMoneyDelta) 0 1 1 "(X=0.000000,Y=0.000000)" "0.000000,0.000000,0.000000")))

(event Custom|CommandAdd
  (Class|InventoryComponent|ExecuteCommand (Variables|Default|GetInven%20Component) (Utilities|Struct|MakeInventoryCommand "Add" (Variables|CommandTestAdd|GetCommand%20Count) (Variables|CommandTestAdd|GetItem%20Data) 1 1 "(X=0.000000,Y=0.000000)" "0.000000,0.000000,0.000000")))

(event Custom|CommandMove
  (Class|InventoryComponent|ExecuteCommand (Variables|Default|GetInven%20Component) (Utilities|Struct|MakeInventoryCommand "Move" 1 0 (Variables|CommandTestMove|GetCommand%20Source%20Index) (Variables|CommandTestMove|GetCommand%20Target%20Index) "(X=0.000000,Y=0.000000)" "0.000000,0.000000,0.000000")))

(event Custom|CommandDrop
  (Class|InventoryComponent|ExecuteCommand (Variables|Default|GetInven%20Component) (Utilities|Struct|MakeInventoryCommand "Drop" 1 0 (Variables|CommandTestDrop|GetDropIndex) (Variables|CommandTestDrop|GetDropIndex) "(X=0.000000,Y=0.000000)" (Transformation|GetActorLocation (Game|Player|GetPlayerPawn 0)))))

(event EventBeginPlay
  (bind _asbp_test_16char_2 (Utilities|Casting|CastToBP_Test16Char2 (Game|Player|GetPlayerPawn 0)))
  (Variables|Default|SetInven%20Component (Variables|/Script/Unreal_Cpp.ActionCharacter|GetInvenComponent _asbp_test_16char_2)))

(fn ConstructionScript)